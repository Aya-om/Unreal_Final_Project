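; BP_Elevator is an interactable platform that the player ball calls to ride up between two height limits.
; Overlapping the trigger enables input and shows the HUD interaction prompt, and pressing Interact while idle starts it rising.
; Leaving the trigger hides the prompt, disables input and sends the platform back down.
; Tick moves the actor vertically by a fixed step per frame, not scaled by delta time, until it reaches a limit.
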(event OnComponentBeginOverlap(Trigger)
  (params (OverlappedComponent :type Primitive%20Component%20Object%20Reference) (OtherActor :type Actor%20Object%20Reference) (OtherComp :type Primitive%20Component%20Object%20Reference) (OtherBodyIndex :type Integer) (bFromSweep :type Boolean) (SweepResult :type Hit%20Result%20Structure%20%28by%20ref%29))
  (Utilities|Casting|CastToBP_Player_Ball OtherActor)
  (Input|EnableInput (Game|GetPlayerController 0))
  (Default|ShowInteractionText (Variables|Default|GetUI%20HUD%20REF)))

(event OnComponentEndOverlap(Trigger)
  (params (OverlappedComponent :type Primitive%20Component%20Object%20Reference) (OtherActor :type Actor%20Object%20Reference) (OtherComp :type Primitive%20Component%20Object%20Reference) (OtherBodyIndex :type Integer))
  (Utilities|Casting|CastToBP_Player_Ball OtherActor)
  (Input|DisableInput (Game|GetPlayerController 0))
  (Default|HideInteractionText (Variables|Default|GetUI%20HUD%20REF))
  (Variables|Default|SetIs%20Moving true)
  (Variables|Default|SetMove%20Up false))

(event EventBeginPlay
  (Utilities|FlowControl|Delay 2.0)
  (bind _asbp_player_ball (Utilities|Casting|CastToBP_Player_Ball (Game|Player|GetPlayerPawn 0)))
  (Variables|Default|SetUI%20HUD%20REF (Variables|/Game/Blueprints/BP_Player_Ball.BP_Player_Ball_C|GetHUD%20REF _asbp_player_ball)))

(event EventTick
  (params (DeltaSeconds :type Float%20%28single-precision%29))
  (bind _returnvalue (Transformation|GetActorLocation))
  (bind _returnvalue_2 (Transformation|GetActorLocation))
  (bind _speed_of_platform (Variables|Default|GetSpeed%20Of%20Platform))
  (bind _speed_of_platform_2 (Variables|Default|GetSpeed%20Of%20Platform))
  (bind _returnvalue_3 (+ (.z _returnvalue_2) _speed_of_platform))
  (bind _returnvalue_4 (- (.z _returnvalue) _speed_of_platform_2))
  (if (Variables|Default|GetIs%20Moving)
    (if (Variables|Default|GetMove%20Up)
      (if (>= _returnvalue_3 (Variables|Default|GetUp%20Limit))
        (Variables|Default|SetIs%20Moving false))
      (Transformation|SetActorLocation (Math|Vector|MakeVector (.x _returnvalue_2) (.y _returnvalue_2) _returnvalue_3) false false)
      (else
        (if (<= _returnvalue_4 (Variables|Default|GetDown%20Limit))
          (Variables|Default|SetIs%20Moving false))
        (Transformation|SetActorLocation (Math|Vector|MakeVector (.x _returnvalue) (.y _returnvalue) _returnvalue_4) false false)))))

(event Input|ActionEvents|InputActionInteract
  (params (Key :type Key%20Structure :default "None"))
  (:Pressed
    (if (not (Variables|Default|GetIs%20Moving))
      (Variables|Default|SetMove%20Up true)
      (Variables|Default|SetIs%20Moving true))))

(fn ConstructionScript)