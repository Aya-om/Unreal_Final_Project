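; BP_Collectable is a spinning coin pickup for the player ball.
; Tick rotates the mesh around yaw by RotationSpeed each frame, without delta-time scaling.
; Overlapping PickUpRadius casts the other actor's Instigator to BP_Player_Ball, plays a coin sound at the pickup's location, increments the player's Coins and destroys the collectable.
; The Volume variable drives both the sound's volume and pitch.
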(event OnComponentBeginOverlap(PickUpRadius)
  (params (OverlappedComponent :type Primitive%20Component%20Object%20Reference) (OtherActor :type Actor%20Object%20Reference) (OtherComp :type Primitive%20Component%20Object%20Reference) (OtherBodyIndex :type Integer) (bFromSweep :type Boolean) (SweepResult :type Hit%20Result%20Structure%20%28by%20ref%29))
  (bind _volume (Variables|Default|Getvolume))
  (bind _asbp_player_ball (Utilities|Casting|CastToBP_Player_Ball (Variables|/Script/Engine.Actor|GetInstigator OtherActor)))
  (Audio|PlaySoundatLocation "/Game/Sounds/mixkit-gold-coin-prize-1999.mixkit-gold-coin-prize-1999" (Transformation|GetActorLocation) "0, 0, 0" _volume _volume 0.0 0 0 0 0)
  (Math|Integer|IncrementInt (Variables|/Game/Blueprints/BP_Player_Ball.BP_Player_Ball_C|GetCoins _asbp_player_ball)
    (:%20%20
      (Actor|DestroyActor))))

(event EventTick
  (params (DeltaSeconds :type Float%20%28single-precision%29))
  (Transformation|AddRelativeRotation (Variables|Default|GetMesh) (Math|Rotator|MakeRotator 0.0 0.0 (Variables|Default|GetRotation%20Speed)) false false))

(fn ConstructionScript)