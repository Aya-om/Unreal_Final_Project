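; BP_Laser is a laser hazard that draws a particle beam and damages the player ball when the beam hits it.
; Every tick it line-traces on the Visibility channel from the actor's location along LaserDirection, up to TraceMaxLength.
; On a hit, it stretches the beam to the impact point and calls PowerDamage on a BP_Player_Ball, so damage repeats each frame of contact.
; Without a hit, the beam endpoints are not updated.
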(event EventTick
  (params (DeltaSeconds :type Float%20%28single-precision%29))
  (bind _returnvalue (Transformation|GetActorLocation))
  (bind (_outhit _returnvalue_2) (Collision|LineTraceByChannel _returnvalue (+ _returnvalue (* (Variables|Default|GetLaser%20Direction) (Variables|Default|GetTrace%20Max%20Length))) "TraceTypeQuery1" false 0 "None"))
  (if _returnvalue_2
    (Class|ParticleSystemComponent|SetBeamSourcePoint (Variables|Default|GetParticleSystem) 0 (Transformation|GetActorLocation))
    (Class|ParticleSystemComponent|SetBeamTargetPoint (Variables|Default|GetParticleSystem) 0 (.Location (Collision|BreakHitResult _outhit)))
    (bind _asbp_player_ball (Utilities|Casting|CastToBP_Player_Ball (.HitActor (Collision|BreakHitResult _outhit))))
    (Default|PowerDamage _asbp_player_ball 5e+01)))

(fn ConstructionScript)